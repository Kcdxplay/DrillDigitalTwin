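; BP_OrbitPlayer is a player-controlled orbit camera that also operates a drill, MainDrill.
; Mouse axes drive control rotation, copied to the SpringArm's relative rotation, while the wheel sets clamped arm length.
; Enhanced Input actions and named events share paths that forward motor movement, stop, speed and placement commands to MainDrill.
; Speed changes broadcast a scaled value through OnRotateSpeedChange, and getter functions expose motor place and moving state.
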(event Custom|SetMotorPlace
  (params (MotorPlace :type Float%20%28double-precision%29))
  (Default|SetMotorPlace (Variables|Default|GetMainDrill) MotorPlace))

(event Custom|MotorMoveUP
  (Default|MoveMotorUp (Variables|Default|GetMainDrill)))

(event Custom|MotorMoveDown
  (Default|MoveMotorDown (Variables|Default|GetMainDrill)))

(event Custom|MotorStop
  (Default|MotorStop (Variables|Default|GetMainDrill)))

(event Custom|MotorSpeedUp
  (bind _maindrill (Variables|Default|GetMainDrill))
  (Default|MotrorSpeedUp _maindrill)
  (bind _newspeed (Default|GetCurrentMotorSpeed _maindrill))
  (Default|CallOnRotateSpeedChange (* _newspeed 2e+02)))

(event Custom|MotorSpeedDown
  (bind _maindrill (Variables|Default|GetMainDrill))
  (Default|MotorSpeedDown _maindrill)
  (bind _newspeed (Default|GetCurrentMotorSpeed _maindrill))
  (Default|CallOnRotateSpeedChange (* _newspeed 2e+02)))

(event Input|EnhancedActionEvents|EnhancedInputActionIA_DrillStop
  (params (ActionValue :type Boolean) (ElapsedSeconds :type Float%20%28double-precision%29) (TriggeredSeconds :type Float%20%28double-precision%29) (InputAction :type Input%20Action%20Object%20Reference :default "/Game/Blueprints/Inputs/IA_DrillStop.IA_DrillStop"))
  (Default|MotorStop (Variables|Default|GetMainDrill)))

(event Input|EnhancedActionEvents|EnhancedInputActionIA_MotorMove
  (params (ActionValue :type Float%20%28double-precision%29) (ElapsedSeconds :type Float%20%28double-precision%29) (TriggeredSeconds :type Float%20%28double-precision%29) (InputAction :type Input%20Action%20Object%20Reference :default "/Game/Blueprints/Inputs/IA_MotorMove.IA_MotorMove"))
  (bind _maindrill (Variables|Default|GetMainDrill))
  (if (>= ActionValue 0.0)
    (Default|MoveMotorUp _maindrill)
    (else
      (Default|MoveMotorDown _maindrill))))

(event Input|EnhancedActionEvents|EnhancedInputActionIA_DrillRotate
  (params (ActionValue :type Float%20%28double-precision%29) (ElapsedSeconds :type Float%20%28double-precision%29) (TriggeredSeconds :type Float%20%28double-precision%29) (InputAction :type Input%20Action%20Object%20Reference :default "/Game/Blueprints/Inputs/IA_DrillRotate.IA_DrillRotate"))
  (bind _maindrill (Variables|Default|GetMainDrill))
  (if (>= ActionValue 0.0)
    (Default|MotrorSpeedUp _maindrill)
    (else
      (Default|MotorSpeedDown _maindrill)))
  (bind _newspeed (Default|GetCurrentMotorSpeed _maindrill))
  (Default|CallOnRotateSpeedChange (* _newspeed 2e+02)))

(event EventBeginPlay)

(event Collision|EventActorBeginOverlap
  (params (OtherActor :type Actor%20Object%20Reference)))

(event EventTick
  (params (DeltaSeconds :type Float%20%28single-precision%29)))

(event Input|MouseEvents|MouseWheelAxis
  (params (AxisValue :type Float%20%28single-precision%29))
  (Variables|/Script/Engine.SpringArmComponent|SetTargetArmLength (Variables|Default|GetSpringArm) (Math|Float|Clamp(Float) (+ (* AxisValue -1.0 (Variables|Default|GetArmAdjustSpeed)) (Variables|/Script/Engine.SpringArmComponent|GetTargetArmLength (Variables|Default|GetSpringArm))) (Variables|Default|GetMinArmLength) (Variables|Default|GetMaxArmLength))))

(event Input|MouseEvents|MouseX
  (params (AxisValue :type Float%20%28single-precision%29))
  ;[1 1 1] 相机旋转控制
  (Pawn|Input|AddControllerYawInput (* AxisValue -1.0 (Variables|Default|GetCmaeraRotateSpeed)))
  (Transformation|SetRelativeRotation (Variables|Default|GetSpringArm) (Pawn|GetControlRotation :!class /Script/Engine.Pawn) false false))

(event Input|MouseEvents|MouseY
  (params (AxisValue :type Float%20%28single-precision%29))
  ;[1 1 1] 相机旋转控制
  (Pawn|Input|AddControllerPitchInput (* AxisValue (Variables|Default|GetCmaeraRotateSpeed)))
  (Transformation|SetRelativeRotation (Variables|Default|GetSpringArm) (Pawn|GetControlRotation :!class /Script/Engine.Pawn) false false))

(fn ConstructionScript)

(fn GetCurrentMotorPlace
  (bind _newparam (Default|GetCurrentMotorPlace (Variables|Default|GetMainDrill)))
  (return _newparam))

(fn GetMotorMovingState
  (return (Variables|/Game/Blueprints/BP_MainDrill.BP_MainDrill_C|GetIsMotorMoving (Variables|Default|GetMainDrill))))