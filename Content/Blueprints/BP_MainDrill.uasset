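; BP_MainDrill is a drill actor with a continuously rotating head and a motor that moves vertically on command.
; A timeline drives the head's yaw from BeginPlay, while MoveMotorUp, MoveMotorDown and MotorStop play, reverse or stop a second timeline.
; SetMotorLocationByPoint maps that timeline's clamped normalized value between the lowest and highest motor heights.
; The construction script sets both play rates, and BeginPlay restores the motor's starting position from CurrentMotorPlace.
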(event Custom|MoveMotorUp
  (bind _motorlocation (Timeline|MotorMoveTimeLine Play)
    (:Update
      (CallFunction|SetMotorLocationbyPoint _motorlocation))))

(event Custom|MoveMotorDown
  (bind _motorlocation (Timeline|MotorMoveTimeLine Reverse)
    (:Update
      (CallFunction|SetMotorLocationbyPoint _motorlocation))))

(event Custom|MotorStop
  (Audio|Components|Audio|Stop (Variables|Default|GetMotorMoveTimeLine)))

(event EventBeginPlay
  (bind _currentmotorplace (Variables|Default|GetCurrentMotorPlace))
  (CallFunction|SetMotorLocationbyPoint _currentmotorplace)
  (Components|Timeline|SetNewTime (Variables|Default|GetMotorMoveTimeLine) _currentmotorplace)
  (bind _rotateplace (Timeline|HeadRotateTimeline Play)
    (:Update
      (Transformation|SetRelativeRotation (Variables|Default|GetHeadMesh) (Math|Rotator|MakeRotator 0.0 0.0 _rotateplace) false false))))

(event Collision|EventActorBeginOverlap
  (params (OtherActor :type Actor%20Object%20Reference)))

(event EventTick
  (params (DeltaSeconds :type Float%20%28single-precision%29)))

(fn ConstructionScript
  (Components|Timeline|SetPlayRate (Variables|Default|GetMotorMoveTimeLine) (Variables|Default|GetMoveSpeedModulus))
  (Components|Timeline|SetPlayRate (Variables|Default|GetHeadRotateTimeline) 5.0))

(fn SetMotorLocationbyPoint
  (params (Point :type Float%20%28double-precision%29))
  (bind _returnvalue (Math|Float|Clamp(Float) Point))
  (bind _lowestmotorlocation (Variables|Default|GetLowestMotorLocation))
  (bind _motormesh (Variables|Default|GetMotorMesh))
  (bind _relativelocation (Variables|/Script/Engine.SceneComponent|GetRelativeLocation _motormesh))
  (Variables|Default|SetCurrentMotorPlace _returnvalue)
  (Transformation|SetRelativeLocation _motormesh (Math|Vector|MakeVector (.x _relativelocation) (.y _relativelocation) (+ (* (- (Variables|Default|GetHighestMotorLocation) _lowestmotorlocation) _returnvalue) _lowestmotorlocation)) false true))