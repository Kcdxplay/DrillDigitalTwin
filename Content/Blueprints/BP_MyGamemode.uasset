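; Game mode for a drill digital-twin app that manages the UI and replays drill data.
; On BeginPlay it caches the player pawn, creates the menu and chart widgets, and shows the cursor.
; DataDistributeComponent buffers the data, and a looping timer dispatches one indexed sample per tick, wrapping at a hardcoded limit.
; Switch events toggle menu opacity and add or remove the gauge container; a DataTable-loading loop is left unconnected.
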(event Custom|DispatchData
  (Class|DataDistributeComponent|DispatchData (Variables|Default|GetDataDistributeComponent) (Utilities|Array|Get(acopy) (Variables|/Script/DrillDDigtalTwins.DataDistributeComponent|GetBuffedDrillData (Variables|Default|GetDataDistributeComponent)) (Variables|Default|GetDrillDataIndex)))
  (bind _result (Math|Integer|IncrementInt (Variables|Default|GetDrillDataIndex))
    (:%20%20
      (if (> _result 4096)
        (Variables|Default|SetDrillDataIndex 0)))))

(event Custom|SwitchToMainMenu
  (Widget|SetRenderOpacity (Variables|Default|GetMainMenuWidget) 1.0)
  (Widget|RemovefromParent (Variables|Default|GetGaugeWidget)))

(event Custom|SwitchToDigitalTwin
  (Widget|SetRenderOpacity (Variables|Default|GetMainMenuWidget) 0.0)
  (UserInterface|Viewport|AddtoViewport (Variables|Default|GetGaugeWidget) 0))

(event EventBeginPlay
  (bind _asbp_main_player (Utilities|Casting|CastToBP_MainPlayer (Game|Player|GetPlayerPawn 0))
    (:then
      (Variables|Default|SetPlayerPawn _asbp_main_player))
    (:CastFailed
      _))
  (CallFunction|SetUpUI)
  (Variables|/Script/Engine.PlayerController|SetbShowMouseCursor (Game|GetPlayerController 0) true)
  (Utilities|Time|SetTimerbyEvent (delegate Custom|DispatchData) 0.1 true)
  (Class|DataDistributeComponent|BuffAllData (Variables|Default|GetDataDistributeComponent)))

(fn ConstructionScript)

(fn SetUpUI
  (bind _returnvalue (UserInterface|CreateWidget "/Game/Widgets/MainMenu_Widget.MainMenu_Widget_C"))
  (bind _output_get (Variables|Default|SetMainMenuWidget _returnvalue))
  (UserInterface|Viewport|AddtoViewport _output_get 0)
  (Utilities|FlowControl|Sequence
    (:then_0
      (bind _returnvalue_2 (UserInterface|CreateWidget "/Game/Widgets/ChartWidgetContainer_Widget.ChartWidgetContainer_Widget_C"))
      (Variables|Default|SetGaugeWidget _returnvalue_2))
    (:then_1
      (bind _returnvalue_3 (UserInterface|CreateWidget "/Game/Widgets/ChartWidget_Line_Widget.ChartWidget_Line_Widget_C"))
      (Variables|Default|SetLineChartWidget _returnvalue_3))))