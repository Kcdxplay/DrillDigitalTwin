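; BP_MainPlayer is a player Blueprint that moves its camera between the ends of a spline.
; BeginPlay places the camera at the spline start; MoveToNextPoint and MoveToPreviousPoint play and reverse a timeline that updates camera location and rotation.
; Updates call GetTranformFromSpline with the timeline alpha, but that function's distance-lerp spline lookups are unconnected.
; Local-space spline rotation is applied as world rotation.
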(event Custom|MoveToNextPoint
  (bind _camera (Variables|Default|GetCamera))
  (bind _movealpha (Timeline|MoveTimeLine Play)
    (:Update
      (Transformation|SetRelativeLocation _camera (.ReturnValue (|GetTranformFromSpline _movealpha)) false false)
      (Transformation|SetWorldRotation _camera (.ReturnValue2 (|GetTranformFromSpline _movealpha)) false false))))

(event Custom|MoveToPreviousPoint
  (bind _camera (Variables|Default|GetCamera))
  (bind _movealpha (Timeline|MoveTimeLine Reverse)
    (:Update
      (Transformation|SetRelativeLocation _camera (.ReturnValue (|GetTranformFromSpline _movealpha)) false false)
      (Transformation|SetWorldRotation _camera (.ReturnValue2 (|GetTranformFromSpline _movealpha)) false false))))

(event EventBeginPlay
  (bind _camera (Variables|Default|GetCamera))
  (bind _spline (Variables|Default|GetSpline))
  (bind _returnvalue (Spline|GetTransformatDistanceAlongSpline _spline 0.0 "Local" false))
  (Transformation|SetRelativeLocation _camera (.location _returnvalue) false false)
  (Transformation|SetWorldRotation _camera (.rotation _returnvalue) false false))

(fn ConstructionScript)